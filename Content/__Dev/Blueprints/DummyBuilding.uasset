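; Placement preview actor for a building that finds compatible BuildingSlot actors and adds itself to the city through one of them.
; On BeginPlay it collects unadded slots with matching Data and shows their highlights, hiding them when destroyed.
; Update targets the nearest candidate within its snap distance and swaps highlight materials; Drop calls AddToCity on that target.
; Tick calls SnapTo, but its cube-lerp logic is disconnected, so no visual snapping occurs.
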(event EventTick
  (params (DeltaSeconds :type Float%20%28single-precision%29))
  (CallFunction|Snapto DeltaSeconds))

(event EventBeginPlay
  (bind _outactors (Actor|GetAllActorsOfClass "/Game/__Dev/Blueprints/BuildingSlot.BuildingSlot_C"))
  (for _array_element _outactors
    (if (== (Variables|Default|GetData) (Variables|/Game/__Dev/Blueprints/BuildingSlot.BuildingSlot_C|GetData _array_element))
      (if (not (Variables|/Game/__Dev/Blueprints/BuildingSlot.BuildingSlot_C|GetAdded _array_element))
        (Utilities|IsValid (Variables|/Game/__Dev/Blueprints/BuildingSlot.BuildingSlot_C|GetHighlight _array_element)
          (:Is%20Valid
            (Utilities|Array|Add (Variables|Default|GetCandidates) _array_element)
            (Development|SetHiddeninGame (Variables|/Game/__Dev/Blueprints/BuildingSlot.BuildingSlot_C|GetHighlight _array_element) false false)
            (Rendering|Material|SetMaterial (Variables|/Game/__Dev/Blueprints/BuildingSlot.BuildingSlot_C|GetHighlight _array_element) 0 "/Game/__Dev/Candidate.Candidate")))))))

(fn ConstructionScript)

(fn ReceiveEndPlay
  (params (EndPlayReason :type EEndPlayReason%20Enum :default "Destroyed"))
  (if (Utilities|Enum|Equal(Enum) EndPlayReason "Destroyed")
    (for _array_element (Variables|Default|GetCandidates)
      (Utilities|IsValid (Variables|/Game/__Dev/Blueprints/BuildingSlot.BuildingSlot_C|GetHighlight _array_element)
        (:Is%20Valid
          (Development|SetHiddeninGame (Variables|/Game/__Dev/Blueprints/BuildingSlot.BuildingSlot_C|GetHighlight _array_element) true false))))))

(fn Update
  (bind _nearest_slot (CallFunction|Sort))
  (CallFunction|UpdateTarget _nearest_slot))

(fn Sort
  (for _array_element (Variables|Default|GetCandidates)
    (bind _output_get (LocalVariables|SetCurrDist (Math|Vector|Distance(Vector) (Transformation|GetActorLocation _array_element) (Transformation|GetActorLocation))))
    (if (< _output_get (LocalVariables|GetMinDist))
      (if (< (LocalVariables|GetCurrDist) (Variables|/Game/__Dev/Blueprints/BuildingSlot.BuildingSlot_C|GetSnapDistance _array_element))
        (LocalVariables|SetMinDist (LocalVariables|GetCurrDist))
        (LocalVariables|SetNearest _array_element))))
  (return (LocalVariables|GetNearest)))

(fn UpdateTarget
  (params (New%20Target :type Building%20Slot%20Object%20Reference))
  (Utilities|IsValid (Variables|Default|GetTarget)
    (:Is%20Valid
      (Rendering|Material|SetMaterial (Variables|/Game/__Dev/Blueprints/BuildingSlot.BuildingSlot_C|GetHighlight (Variables|Default|GetTarget)) 0 "/Game/__Dev/Candidate.Candidate"))
    (:Is%20Not%20Valid
      _))
  (if (!= New%20Target (Variables|Default|GetTarget))
    (Variables|Default|SetT 0.0))
  (bind _output_get (Variables|Default|SetTarget New%20Target))
  (Utilities|IsValid _output_get
    (:Is%20Valid
      (Rendering|Material|SetMaterial (Variables|/Game/__Dev/Blueprints/BuildingSlot.BuildingSlot_C|GetHighlight _output_get) 0 "/Game/__Dev/Place.Place"))))

(fn Snapto
  (params (DeltaTime :type Float%20%28double-precision%29)))

(fn Drop
  (bind _target (Variables|Default|GetTarget))
  (Utilities|IsValid _target
    (:Is%20Valid
      (Default|AddtoCity _target))))