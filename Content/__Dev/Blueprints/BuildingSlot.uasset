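; BuildingSlot is a placement slot for a city building, revealing or hiding its TargetActors as the building is added or removed.
; AddToCity triggers the pawn's placement animation, then after a delay unhides the targets and updates props, while Tick grows their Z scale, including instanced foliage.
; RemoveFromCity hides targets immediately and recurses into nested slots.
; The construction script derives highlight, snap sphere and label from BaseSize and Data.
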(event Custom|AddToCity
  (Input|SetInputModeGameOnly (Game|GetPlayerController 0) true)
  (bind _aspawn_blueprint (Utilities|Casting|CastToPawn_Blueprint (Game|Player|GetPlayerPawn 0)))
  (Default|AnimatePlacement _aspawn_blueprint self)
  (Utilities|FlowControl|Delay 1.0)
  (Variables|Default|SetAdded true)
  (for _array_element (Variables|Default|GetTargetActors)
    (Utilities|IsValid _array_element
      (:Is%20Valid
        (Rendering|SetActorHiddenInGame _array_element false))))
  (Default|UpdateProps _aspawn_blueprint))

(event EventBeginPlay
  (for _array_element (Variables|Default|GetTargetActors)
    (Utilities|IsValid _array_element
      (:Is%20Valid
        (Rendering|SetActorHiddenInGame _array_element true)))))

(event EventTick
  (params (DeltaSeconds :type Float%20%28single-precision%29))
  (bind _output_get (Variables|Default|SetSize (Math|Float|Clamp(Float) (+ (Variables|Default|GetSize) (* DeltaSeconds (Variables|Default|GetSpeed) (Math|Float|SelectFloat 1.0 -1.0 (Variables|Default|GetAdded)))))))
  (for _array_element (Variables|Default|GetTargetActors)
    (Transformation|SetActorScale3D _array_element (Math|Vector|MakeVector 1.0 1.0 _output_get))
    (for _array_element_2 (Actor|GetComponentsByClass _array_element "/Script/Foliage.FoliageInstancedStaticMeshComponent")
      (Transformation|SetRelativeScale3D _array_element_2 (Math|Vector|MakeVector 1.0 1.0 _output_get)))))

(fn ConstructionScript
  (bind _basesize (Variables|Default|GetBaseSize))
  (bind (_x _y) (Math|Vector|BreakVector _basesize))
  (Transformation|SetRelativeScale3D (Variables|Default|GetHighlight) _basesize)
  (Variables|Default|SetSnapDistance (* (Math|Vector2D|Vector2DLength (Math|Vector2D|MakeVector2D _x _y)) 5e+02))
  (Components|Sphere|SetSphereRadius (Variables|Default|GetSphere) (Variables|Default|GetSnapDistance) true)
  (Rendering|Components|TextRender|SetText (Variables|Default|GetTextRender) (Utilities|Text|ToText(String) (Utilities|String|Replace (Utilities|GetObjectName (Variables|Default|GetData)) "_" " "))))

(fn RemovefromCity
  (params (Nested :type Boolean))
  (Variables|Default|SetAdded false)
  (for _array_element (Variables|Default|GetTargetActors)
    (Utilities|IsValid _array_element
      (:Is%20Valid
        (Rendering|SetActorHiddenInGame _array_element true)
        (bind _asbuilding_slot (Utilities|Casting|CastToBuildingSlot _array_element))
        (CallFunction|RemovefromCity _asbuilding_slot true))))
  (if (not Nested)
    (bind _aspawn_blueprint (Utilities|Casting|CastToPawn_Blueprint (Game|Player|GetPlayerPawn 0)))
    (Default|UpdateProps _aspawn_blueprint)))